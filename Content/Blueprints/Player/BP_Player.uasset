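; Player Blueprint that lets the user place and select BP_PlacedActor objects with the right mouse button.
; Each click unflags the current selection, then traces under the cursor to select the placed actor hit or spawn a new one there.
; New actors take the mesh from BP_PlayerState and are offset by its local bounds maximum.
; ChangeCurrentSelectionActor stores the selection in BP_PlayerState, flags it and updates the main UI.
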(event `Key|RightMouseButton`
  (params (Key :type "Key Structure"))
  (bind _hitresult (`PlayerController.GetHitResultUnderCursorByChannel` (`GameplayStatics.GetPlayerController` 0) "TraceTypeQuery1" true))
  (:`Pressed`
    (`|ExecutionSequence`
      (:`then_0`
        ;[1 1 1] First of all, Check if Player has selection.
        (bind _asbp_player_state (cast `/Game/Blueprints/State/BP_PlayerState` (`self.PlayerState`)))
        (bind _currentcarryobj (`/Game/Blueprints/State/BP_PlayerState.CurrentCarryObj` _asbp_player_state))
        (`/Engine/EditorBlueprintResources/StandardMacros.IsValid` _currentcarryobj
          (:`Is Valid`
            (`/Game/Blueprints/Utility/BP_PlacedActor.IsChangeByPlayer` _currentcarryobj false))))
      (:`then_1`
        (if (`GameplayStatics.BreakHitResult` _hitresult)
          (bind _asbp_placed_actor (cast `/Game/Blueprints/Utility/BP_PlacedActor` (`.HitActor` (`GameplayStatics.BreakHitResult` _hitresult)))
            (:`then`
              (`self.ChangeCurrentSelectionActor` _asbp_placed_actor) ; Just select it
            )
            (:`CastFailed`
              ;[1 1 1] New Object spawn.
              (bind _returnvalue (`|SpawnActorFromClass` "/Game/Blueprints/Utility/BP_PlacedActor.BP_PlacedActor_C" (`KismetMathLibrary.MakeTransform` (`.Location` (`GameplayStatics.BreakHitResult` _hitresult))) "Undefined" "OverrideRootScale" null null))
              (`StaticMeshComponent.SetStaticMesh` (`/Game/Blueprints/Utility/BP_PlacedActor.StaticMesh` _returnvalue) (`/Game/Blueprints/State/BP_PlayerState.CurrentStaticMeshObject` _asbp_player_state))
              (`self.ChangeCurrentSelectionActor` _returnvalue)
              (`self.K2_AddActorLocalOffset` _returnvalue (`.Max` (`StaticMeshComponent.GetLocalBounds` (`/Game/Blueprints/Utility/BP_PlacedActor.StaticMesh` _returnvalue))) false false))))))))

(fn `ChangeCurrentSelectionActor`
  (params (CurrentCarryObj :type "/Game/Blueprints/Utility/BP_PlacedActor Object Reference"))
  (bind _asbp_player_state (cast `/Game/Blueprints/State/BP_PlayerState` (`self.PlayerState`)))
  (bind _output_get (set `/Game/Blueprints/State/BP_PlayerState.CurrentCarryObj` CurrentCarryObj _asbp_player_state))
  (`/Game/Blueprints/Utility/BP_PlacedActor.IsChangeByPlayer` _output_get true)
  (`/Game/Blueprints/UI/BP_PlacedUI.ChangeCurrentObject` (`/Game/Blueprints/State/BP_PlayerState.PlayerMainUiInstance` _asbp_player_state) _output_get))

(fn `UserConstructionScript`)