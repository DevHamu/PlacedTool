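; BP_PlayerController is the player controller that sets up the main on-screen UI and handles quitting the game.
; On BeginPlay it creates the BP_PlacedUI widget, adds it to the viewport, shows the mouse cursor and switches to Game and UI input.
; It then stores the widget on BP_PlayerState as the main UI instance.
; Pressing Escape quits the game.
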(event `self.ReceiveBeginPlay`
  ;[1 1 1] Spawn UI and hold it until game is quited
  (bind _returnvalue (`|CreateWidget` "/Game/Blueprints/UI/BP_PlacedUI.BP_PlacedUI_C"))
  (`UserWidget.AddToViewport` _returnvalue 0)
  (set `self.bShowMouseCursor` true)
  (`WidgetBlueprintLibrary.SetInputMode_GameAndUIEx` (`GameplayStatics.GetPlayerController` 0) null)
  (bind _asbp_player_state (cast `/Game/Blueprints/State/BP_PlayerState` (`self.PlayerState`)))
  (set `/Game/Blueprints/State/BP_PlayerState.PlayerMainUiInstance` _returnvalue _asbp_player_state))

(event `Key|Escape`
  (params (Key :type "Key Structure"))
  ;[1 1 1] Quit game
  (:`Pressed`
    (`KismetSystemLibrary.QuitGame` (`GameplayStatics.GetPlayerController` 0) "Quit")))

(fn `UserConstructionScript`)